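; BP_Hat is a hat that can be worn by a character or dropped as a loose physics object.
; AttachHat stores the character as owner, turns off the static mesh's physics and collision, then snaps it to the character mesh's "Hat" socket, keeping world scale.
; DetachHat clears the owner, restores collision and physics, and detaches the mesh in place.
; Event graph and construction script are empty.
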(event EventBeginPlay)

(event Collision|EventActorBeginOverlap
  (params (OtherActor :type Actor%20Object%20Reference)))

(event EventTick
  (params (DeltaSeconds :type Float%20%28single-precision%29)))

(fn ConstructionScript)

(fn AttachHat
  (params (Charactor :type Character%20Object%20Reference))
  (Variables|Default|SetOwnCharacter Charactor)
  (Physics|SetSimulatePhysics (Variables|Default|GetStaticMesh) false)
  (Collision|SetCollisionEnabled (Variables|Default|GetStaticMesh) "NoCollision")
  (Transformation|AttachComponentToComponent (Variables|/Script/Engine.Character|GetMesh Charactor) "Hat" "SnapToTarget" "SnapToTarget" "KeepWorld" true)
  (return false))

(fn DetachHat
  (bind _staticmesh (Variables|Default|GetStaticMesh))
  (Variables|Default|SetOwnCharacter 0)
  (Collision|SetCollisionEnabled _staticmesh "QueryAndPhysics")
  (Physics|SetSimulatePhysics _staticmesh true)
  (Transformation|DetachFromComponent (Variables|Default|GetStaticMesh) "KeepWorld" "KeepWorld" "KeepWorld" true)
  (return false))