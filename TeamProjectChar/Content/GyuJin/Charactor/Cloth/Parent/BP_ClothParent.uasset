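; BP_ClothParent is a parent Blueprint for wearable clothing that can be attached to and dropped from a character.
; AttachCloth stores the wearer, disables physics and collision, snaps to the "Cloth" socket and applies ABP_Bunny animation.
; DetachCloth clears the wearer, re-enables physics and collision, and detaches in world space.
; Jump input is forwarded to the stored wearer, while the hat attach and detach functions are stubs returning false.
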(event EventBeginPlay)

(event Collision|EventActorBeginOverlap
  (params (OtherActor :type Actor%20Object%20Reference)))

(event EventTick
  (params (DeltaSeconds :type Float%20%28single-precision%29)))

(event Input|ActionEvents|InputActionJump
  (params (Key :type Key%20Structure :default "None"))
  (bind _owncharacter (Variables|Default|GetOwnCharacter))
  (:Pressed
    (Character|Jump _owncharacter))
  (:Released
    (Character|StopJumping _owncharacter)))

(fn ConstructionScript)

(fn AttachCloth
  (params (Charactor :type Character%20Object%20Reference))
  (bind _skeletalmesh (Variables|Default|GetSkeletalMesh))
  (Variables|Default|SetOwnCharacter Charactor)
  (Physics|SetSimulatePhysics _skeletalmesh false)
  (Collision|SetCollisionEnabled _skeletalmesh "NoCollision")
  (Transformation|AttachComponentToComponent (Variables|/Script/Engine.Character|GetMesh Charactor) "Cloth" "SnapToTarget" "SnapToTarget" "KeepWorld" true)
  (Class|SkeletalMeshComponent|SetAnimClass (Variables|Default|GetSkeletalMesh) "/Game/GyuJin/Charactor/Bunny/Mesh/ABP_Bunny.ABP_Bunny_C")
  (return false))

(fn AttachHat
  (params (Charactor :type Character%20Object%20Reference))
  (return false))

(fn DetachCloth
  (bind _skeletalmesh (Variables|Default|GetSkeletalMesh))
  (Variables|Default|SetOwnCharacter 0)
  (Collision|SetCollisionEnabled _skeletalmesh "QueryAndPhysics")
  (Physics|SetSimulatePhysics _skeletalmesh true)
  (Transformation|DetachFromComponent _skeletalmesh "KeepWorld" "KeepWorld" "KeepWorld" true)
  (return false))

(fn DetachHat
  (return false))