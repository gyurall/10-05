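; BP_PawnPiggy is the Piggy animal pawn, with a slide ability that runs on MP stored in its AnimalState player state.
; Each Tick while sliding, it calls UseMPSlide with a frame-time-scaled cost; a true result disables sliding and sets walk speed to a fixed value.
; Otherwise it calls GetMPSlide with the same scaled amount, and a true result allows sliding again.
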(event EventTick
  (params (DeltaSeconds :type Float%20%28single-precision%29))
  (bind _returnvalue (Utilities|Time|GetWorldDeltaSeconds))
  (bind _mp_usesizeofslide (Variables|Default|GetMP_UseSizeOfSlide))
  (bind _returnvalue_2 (* _mp_usesizeofslide _returnvalue))
  ;[1 1 1] UseMP
  (if (Variables|Default|GetIsSlide)
    (bind _asanimal_state (Utilities|Casting|CastToAnimalState (Variables|Default|GetPlayerState)))
    (bind _isnull (Default|UseMPSlide _asanimal_state _returnvalue_2))
    (if _isnull
      (Variables|Default|SetCanSlide false)
      (Variables|/Script/Engine.CharacterMovementComponent|SetMaxWalkSpeed (Variables|Character|GetCharacterMovement) 6e+02))
    (else
      (bind _asanimal_state_2 (Utilities|Casting|CastToAnimalState (Variables|Default|GetPlayerState)))
      (bind _ismor20 (Default|GetMPSlide _asanimal_state_2 _returnvalue_2))
      (if _ismor20
        (Variables|Default|SetCanSlide true)))))

(fn ConstructionScript)